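; Grind collision Blueprint that produces spark effects while it is in contact with a surface.
; Each tick it sphere-traces a short distance downward, using the radius that also sizes its collision sphere in construction.
; On a hit it aligns the grind VFX to the surface normal, activates it, sets light visibility and starts playback once.
; Losing contact resets the one-shot, deactivates the effect, updates visibility and stops playback.
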(event EventTick
  (params (DeltaSeconds :type Float%20%28single-precision%29))
  (bind _returnvalue (Transformation|GetWorldLocation))
  (bind (_outhit _returnvalue_2) (Collision|SphereTraceForObjects _returnvalue (+ _returnvalue "0.000000,0.000000,-20.000000") (Variables|Effect|GetCollisionSphere) (|CollapseGraph_0) false 0 "None"))
  (if _returnvalue_2
    (Transformation|SetWorldRotation (Variables|Default|GetVFX_GrindNoLight) (Math|Rotator|MakeRotationfromAxes (.Normal (Collision|BreakHitResult _outhit)) "0, 0, 0" "0, 0, 0") false)
    (Components|Activation|Activate false)
    (Rendering|SetVisibility (Variables|Default|GetLightOn) false)
    (|DoOnceMultiInput :!label _label
      (:A%20Out
        (Audio|Components|Audio|Play 0.0)))
    (else
      (Utilities|FlowControl|Sequence
        (:then_0
          (goto _label Reset%20In))
        (:then_1
          (Components|Activation|Deactivate)
          (Rendering|SetVisibility (Variables|Default|GetLightOff) false)
          (Audio|Components|Audio|Stop))))))

(fn ConstructionScript
  (Components|Sphere|SetSphereRadius (Variables|Default|GetGrindCollision) (Variables|Effect|GetCollisionSphere) true))